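; Turret actor that fires target-seeking projectiles at the TopDownCharacter and can be destroyed by damage.
; Entering PissOffRadius fires immediately and starts a one-second looping timer, handing each projectile the player's capsule as target.
; Leaving GTFO_Radius clears the timer with a zero-time call and resets the DoOnce.
; Damage spawns an explosion; at zero health a short-delay loop sinks the turret until it is destroyed.
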(event `self.PissOffRadius.OnComponentBeginOverlap`
  (params (OverlappedComponent :type "PrimitiveComponent Object Reference") (OtherActor :type "Actor Object Reference") (OtherComp :type "PrimitiveComponent Object Reference") (OtherBodyIndex :type Integer) (bFromSweep :type Boolean) (SweepResult :type "HitResult Structure (by ref)"))
  ;[1 1 1] Entrée dans la range
  (bind _astop_down_character (cast `/Game/TopDownBP/Blueprints/TopDownCharacter` OtherActor))
  (set `self.InRange` true)
  (set `self.ProjectileTarget` (`Character.CapsuleComponent` _astop_down_character))
  (`/Engine/EditorBlueprintResources/StandardMacros.DoOnce` false :!label _label
    (:`Completed`
      ;[1 1 1] Création du projectile et visée auto
      (`KismetSystemLibrary.K2_SetTimerDelegate` (delegate `Fire`) 1.0 true)
      (bind _returnvalue (`|SpawnActorFromClass` "/Game/Turret/ProjectileTurret_BP.ProjectileTurret_BP_C" (`KismetMathLibrary.Conv_VectorToTransform` (`SceneComponent.K2_GetComponentLocation` (`self.ShootPoint`))) "AdjustIfPossibleButAlwaysSpawn" "OverrideRootScale" null null :!label _label_2))
      (bind _asprojectile_turret_bp (cast `/Game/Turret/ProjectileTurret_BP` _returnvalue))
      (set `/Game/Turret/ProjectileTurret_BP.MyTarget` (`self.ProjectileTarget`) _asprojectile_turret_bp))))

(event `self.GTFO_Radius.OnComponentEndOverlap`
  (params (OverlappedComponent :type "PrimitiveComponent Object Reference") (OtherActor :type "Actor Object Reference") (OtherComp :type "PrimitiveComponent Object Reference") (OtherBodyIndex :type Integer))
  ;[1 1 1] Sortie de la range
  (cast `/Game/TopDownBP/Blueprints/TopDownCharacter` OtherActor)
  (set `self.InRange` false)
  (`KismetSystemLibrary.K2_SetTimerDelegate` (delegate `Fire`))
  (goto _label :!via `Reset`))

(event `Fire`
  ;[1 1 1] Sortie de la range
  (goto _label_2))

(event `self.ReceiveAnyDamage`
  (params (Damage :type "Float (single-precision)") (DamageType :type "DamageType Object Reference") (InstigatedBy :type "Controller Object Reference") (DamageCauser :type "Actor Object Reference"))
  (bind _returnvalue (`self.K2_GetActorLocation`))
  ;[1 0.102 0.1617] Dégats/Mort
  (set `self.Health` (- (`self.Health`) Damage))
  (`GameplayStatics.SpawnEmitterAtLocation` "/Game/StarterContent/Particles/P_Explosion.P_Explosion" _returnvalue (struct) (3.0 3.0 3.0))
  (if (<= (`self.Health`) 0.0)
    (`self.K2_SetActorLocation` (+ _returnvalue (0.0 0.0 -10.0)) true :!label _label_3)
    (`|ExecutionSequence`
      (:`then_0`
        (`KismetSystemLibrary.Delay` 1.0)
        (`self.K2_DestroyActor`)
        (`KismetSystemLibrary.PrintString` "Tour détruite"))
      (:`then_1`
        (`KismetSystemLibrary.Delay` 0.01)
        (goto _label_3)))))

(fn `UserConstructionScript`)